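; BP_SwarmGamemode is the game mode that bootstraps the swarm game's core actors and HUD on BeginPlay.
; It finds the player character, wave manager and enemy minions manager in the level and calls Init on each with itself.
; A second PostInit pass then hands all three references to each, so cross-references are set after initialization.
; Finally it creates UI_HUD, initializes it with itself and the wave manager, and adds it to the viewport.
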(event EventBeginPlay
  (Utilities|FlowControl|Sequence
    (:then_0
      (bind _returnvalue (Actor|GetActorOfClass "/Game/Blueprints/Player/BP_PlayerCharacter.BP_PlayerCharacter_C"))
      (Utilities|IsValid _returnvalue
        (:Is%20Valid
          (bind _output_get (Variables|Default|SetPlayerChar _returnvalue))
          (Default|Init _output_get self))))
    (:then_1
      (bind _returnvalue_2 (Actor|GetActorOfClass "/Game/Blueprints/Wave/BP_WaveManager.BP_WaveManager_C"))
      (Utilities|IsValid _returnvalue_2
        (:Is%20Valid
          (Default|Init _returnvalue_2 self)
          (Variables|Default|SetWaveManager _returnvalue_2))))
    (:then_2
      (bind _returnvalue_3 (Actor|GetActorOfClass "/Game/Blueprints/Enemies/BP_EnemyMinionsManager.BP_EnemyMinionsManager_C"))
      (Utilities|IsValid _returnvalue_3
        (:Is%20Valid
          (Default|Init _returnvalue_3 self)
          (Variables|Default|SetEnemyMinionsManager _returnvalue_3))))
    (:then_3
      (Default|PostInit (Variables|Default|GetPlayerChar) (Variables|Default|GetPlayerChar) (Variables|Default|GetWaveManager) (Variables|Default|GetEnemyMinionsManager))
      (Default|PostInit (Variables|Default|GetWaveManager) (Variables|Default|GetPlayerChar) (Variables|Default|GetWaveManager) (Variables|Default|GetEnemyMinionsManager))
      (Default|PostInit (Variables|Default|GetEnemyMinionsManager) (Variables|Default|GetPlayerChar) (Variables|Default|GetWaveManager) (Variables|Default|GetEnemyMinionsManager)))
    (:then_4
      (bind _returnvalue_4 (UserInterface|CreateWidget "/Game/UI/UI_HUD.UI_HUD_C"))
      (Variables|Default|SetHUD _returnvalue_4)
      (Default|Init _returnvalue_4 self (Variables|Default|GetWaveManager))
      (UserInterface|Viewport|AddtoViewport _returnvalue_4 0))))

(fn ConstructionScript)