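; BP_PlayerCharacter is a god-view player character that commands a minion wave through WaveManager.
; Input pans and rotates the spring-arm camera, with zoom also remapping its pitch.
; Mouse-cursor traces set the wave's movement target or pick up passive items for it; selecting enemies has no effect yet.
; Init events inject the game mode and managers, while other inputs toggle auto-attack and debug-spawn or kill minions.
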(event Input|EnhancedActionEvents|EnhancedInputActionIA_GodMove
  (params (ActionValue :type Vector%202D%20Structure) (ElapsedSeconds :type Float%20%28double-precision%29) (TriggeredSeconds :type Float%20%28double-precision%29) (InputAction :type Input%20Action%20Object%20Reference :default "/Game/Input/Actions/IA_GodMove.IA_GodMove"))
  (bind _springarm (Variables|Default|GetSpringArm))
  (bind _returnvalue (Class|SpringArmComponent|GetTargetRotation _springarm))
  (Pawn|Input|AddMovementInput (+ (* (.y ActionValue) (Math|Vector|GetRightVector _returnvalue)) (* (.x ActionValue) (Math|Vector|GetForwardVector _returnvalue))) 1.0 false))

(event Input|EnhancedActionEvents|EnhancedInputActionIA_Move
  (params (ActionValue :type Boolean) (ElapsedSeconds :type Float%20%28double-precision%29) (TriggeredSeconds :type Float%20%28double-precision%29) (InputAction :type Input%20Action%20Object%20Reference :default "/Game/Input/Actions/IA_Move.IA_Move"))
  (bind _returnvalue (Game|GetPlayerController 0))
  (bind (_worldlocation _worlddirection) (Game|Player|ConvertMouseLocationToWorldSpace _returnvalue))
  (bind _outhit (Collision|LineTraceByChannel _worldlocation (+ _worldlocation (* _worlddirection 5e+04)) "TraceTypeQuery1" false 0 "None"))
  (Default|SetMovementTarget (Variables|References|GetWaveManager) (.Location (Collision|BreakHitResult _outhit))))

(event Input|EnhancedActionEvents|EnhancedInputActionIA_GodRotate
  (params (ActionValue :type Float%20%28double-precision%29) (ElapsedSeconds :type Float%20%28double-precision%29) (TriggeredSeconds :type Float%20%28double-precision%29) (InputAction :type Input%20Action%20Object%20Reference :default "/Game/Input/Actions/IA_GodRotate.IA_GodRotate"))
  (bind _springarm (Variables|Default|GetSpringArm))
  (bind _relativerotation (Variables|/Script/Engine.SceneComponent|GetRelativeRotation _springarm))
  ;[0.15 0.15 0.15 0.5] Camera
  (Transformation|SetRelativeRotation _springarm (Math|Rotator|MakeRotator (.roll _relativerotation) (.pitch _relativerotation) (+ ActionValue (.yaw _relativerotation))) false false))

(event Input|EnhancedActionEvents|EnhancedInputActionIA_ToggleMoveMode
  (params (ActionValue :type Boolean) (ElapsedSeconds :type Float%20%28double-precision%29) (TriggeredSeconds :type Float%20%28double-precision%29) (InputAction :type Input%20Action%20Object%20Reference :default "/Game/Input/Actions/IA_ToggleMoveMode.IA_ToggleMoveMode"))
  (:Started
    (bind _isa (Utilities|FlowControl|FlipFlop)
      (:A
        _)
      (:B
        _))
    (Default|ToggleAutoAttack (Variables|References|GetWaveManager) _isa)))

(event Input|EnhancedActionEvents|EnhancedInputActionIA_DEBUG_SpawnMinion
  (params (ActionValue :type Boolean) (ElapsedSeconds :type Float%20%28double-precision%29) (TriggeredSeconds :type Float%20%28double-precision%29) (InputAction :type Input%20Action%20Object%20Reference :default "/Game/Input/Actions/Debug/IA_DEBUG_SpawnMinion.IA_DEBUG_SpawnMinion"))
  ;[0.15 0.15 0.15 0.5] Debug
  (:Started
    (Default|AddMinion (Variables|References|GetWaveManager))))

(event Input|EnhancedActionEvents|EnhancedInputActionIA_DEBUG_KillMinion
  (params (ActionValue :type Boolean) (ElapsedSeconds :type Float%20%28double-precision%29) (TriggeredSeconds :type Float%20%28double-precision%29) (InputAction :type Input%20Action%20Object%20Reference :default "/Game/Input/Actions/Debug/IA_DEBUG_KillMinion.IA_DEBUG_KillMinion"))
  (bind _wavemanager (Variables|References|GetWaveManager))
  ;[0.15 0.15 0.15 0.5] Debug
  (:Started
    (Default|RemoveMinion _wavemanager (.OutItem (Utilities|Array|Random (Variables|/Game/Blueprints/Wave/BP_WaveManager.BP_WaveManager_C|GetMinions _wavemanager))))))

(event Input|EnhancedActionEvents|EnhancedInputActionIA_Select
  (params (ActionValue :type Boolean) (ElapsedSeconds :type Float%20%28double-precision%29) (TriggeredSeconds :type Float%20%28double-precision%29) (InputAction :type Input%20Action%20Object%20Reference :default "/Game/Input/Actions/IA_Select.IA_Select"))
  (bind _returnvalue (Game|GetPlayerController 0))
  (bind (_worldlocation _worlddirection) (Game|Player|ConvertMouseLocationToWorldSpace _returnvalue))
  (:Started
    (bind (_outhit _returnvalue_2) (Collision|LineTraceForObjects _worldlocation (+ _worldlocation (* _worlddirection 5e+04)) (Utilities|Array|MakeArray "ObjectTypeQuery8" "ObjectTypeQuery9") false 0 "None"))
    (if _returnvalue_2
      (Utilities|FlowControl|Sequence
        (:then_0
          (bind _asbp_passive_item (Utilities|Casting|CastToBP_PassiveItem (.HitActor (Collision|BreakHitResult _outhit))))
          (Default|PickUp _asbp_passive_item)
          (Default|AddPassiveItem (Variables|References|GetWaveManager) (Variables|/Game/Blueprints/Items/BP_PassiveItem.BP_PassiveItem_C|GetPassiveItem _asbp_passive_item)))
        (:then_1
          (Utilities|Casting|CastToBP_EnemyChar (.HitActor (Collision|BreakHitResult _outhit))))))))

(event Input|EnhancedActionEvents|EnhancedInputActionIA_GodZoom
  (params (ActionValue :type Float%20%28double-precision%29) (ElapsedSeconds :type Float%20%28double-precision%29) (TriggeredSeconds :type Float%20%28double-precision%29) (InputAction :type Input%20Action%20Object%20Reference :default "/Game/Input/Actions/IA_GodZoom.IA_GodZoom"))
  (bind _defaultarmlength (Variables|Default|GetDefaultArmLength))
  (bind _springarm (Variables|Default|GetSpringArm))
  (bind _relativerotation (Variables|/Script/Engine.SceneComponent|GetRelativeRotation _springarm))
  ;[0.15 0.15 0.15 0.5] Camera
  (Variables|/Script/Engine.SpringArmComponent|SetTargetArmLength _springarm (Math|Float|Clamp(Float) (+ (* (* ActionValue -1.0) 1e+02) (Variables|/Script/Engine.SpringArmComponent|GetTargetArmLength (Variables|Default|GetSpringArm))) 0.0 _defaultarmlength))
  (Transformation|SetRelativeRotation _springarm (Math|Rotator|MakeRotator (.roll _relativerotation) (Math|Float|MapRangeClamped (Math|Float|Clamp(Float) (+ (* (* ActionValue -1.0) 1e+02) (Variables|/Script/Engine.SpringArmComponent|GetTargetArmLength (Variables|Default|GetSpringArm))) 0.0 _defaultarmlength) 1e+02 _defaultarmlength 5.0 -4e+01) (.yaw _relativerotation)) false false))

(event EventInit
  (params (GameMode :type BP%20Swarm%20Gamemode%20Object%20Reference))
  (Variables|References|SetGameMode GameMode))

(event EventPostInit
  (params (PlayerCharacter :type BP%20Player%20Character%20Object%20Reference) (WaveManager :type BP%20Wave%20Manager%20Object%20Reference) (EnemyMinionsManager :type BP%20Enemy%20Minions%20Manager%20Object%20Reference) (ChampsManager :type Object%20Object%20Reference))
  (Variables|References|SetWaveManager WaveManager)
  (Variables|References|SetEnemyMinionsManager EnemyMinionsManager))

(fn ConstructionScript)