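; Base unit actor that fights tagged enemies, with stat-scaled movement speed, attack damage and attack rate.
; AI perception tracks sensed enemies in a map and writes AutoAttackTarget to the Blackboard, switching to the closest when the target is lost.
; Attacks go through BI_Attackable, with a delay clearing the attacking flag.
; Damage shows on a widget and fires OnUnitDeath at zero life, while Kill separately handles effect and destruction.
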(event OnTargetPerceptionInfoUpdated(AIPerception)
  (params (UpdateInfo :type Actor%20Perception%20Update%20Info%20Structure%20%28by%20ref%29))
  (bind (_targetid _target _stimulus) (Utilities|Struct|BreakActorPerceptionUpdateInfo UpdateInfo))
  (if (Utilities|Struct|BreakAIStimulus _stimulus)
    (if (CallFunction|IsAnEnemy _target)
      (Utilities|Map|Add (Variables|Default|GetSurroundingEnemies) _targetid _target)
      (if (== (Variables|Default|GetLastPerceptionTarget) -1)
        (Variables|Default|SetLastPerceptionTarget _targetid)
        (AI|Components|Blackboard|SetValueasObject (AI|GetBlackboard 0) (Utilities|Name|MakeLiteralName "AutoAttackTarget") _target)))
    (else
      (Utilities|Map|Remove (Variables|Default|GetSurroundingEnemies) _targetid)
      (if (== _targetid (Variables|Default|GetLastPerceptionTarget))
        (if (Utilities|Map|IsNotEmpty (Variables|Default|GetSurroundingEnemies))
          (Variables|Default|SetLastPerceptionTarget (.EnemyID (CallFunction|FindClosestEnemy)))
          (AI|Components|Blackboard|SetValueasObject (AI|GetBlackboard 0) (Utilities|Name|MakeLiteralName "AutoAttackTarget") (.Value (Utilities|Map|Find (Variables|Default|GetSurroundingEnemies) (Variables|Default|GetLastPerceptionTarget))))
          (else
            (Variables|Default|SetLastPerceptionTarget -1)
            (AI|Components|Blackboard|SetValueasObject (AI|GetBlackboard 0) (Utilities|Name|MakeLiteralName "AutoAttackTarget") 0)))))))

(event EventAttack
  (params (Target :type BI%20Attackable%20Interface))
  (bind _stats (Variables|Default|GetStats))
  (bind (_attackspeed _attackdamage) (Utilities|Struct|BreakST_UnitStats _stats))
  (bind _asbi_attackable (Utilities|Casting|CastToBI_Attackable Target))
  (Variables|Default|SetIsAttacking true)
  (Default|ReceiveDamage _asbi_attackable (* _attackdamage (Variables|Default|GetBaseAttackDamage)) self)
  (Utilities|FlowControl|Delay (/ 1.0 (+ (/ _attackspeed 100) (Variables|Default|GetAttacksPerSecond))))
  (Variables|Default|SetIsAttacking false))

(event EventInit
  (params (Stats :type ST%20Unit%20Stats%20Structure))
  (CallFunction|UpdateStats Stats))

(event EventDamage
  (params (Damage :type Float%20%28double-precision%29) (DamageSource :type BP%20Unit%20Object%20Reference))
  (bind _output_get (Variables|Default|SetLife (- (Variables|Default|GetLife) Damage)))
  (Default|ShowDamage (Variables|Default|GetDamageDisplayer) Damage)
  (if (<= _output_get 0.0)
    (Default|CallOnUnitDeath self DamageSource)))

(event EventKill
  (Effects|SpawnEmitteratLocation "/Game/FXVarietyPack/Particles/P_ky_hit2.P_ky_hit2" (Transformation|GetActorLocation))
  (Actor|DestroyActor))

(event EventBeginPlay
  (bind _asui_damage_displayer (Utilities|Casting|CastToUI_DamageDisplayer (UserInterface|GetUserWidgetObject (Variables|Default|GetWidget))))
  (Variables|Default|SetDamageDisplayer _asui_damage_displayer))

(event EventUpdateStats
  (params (NewStats :type ST%20Unit%20Stats%20Structure))
  (bind _returnvalue (AI|GetBlackboard 0))
  (bind _output_get (Variables|Default|SetStats NewStats))
  (Utilities|IsValid _returnvalue
    (:Is%20Valid
      (AI|Components|Blackboard|SetValueasFloat _returnvalue (Utilities|Name|MakeLiteralName "AttackCooldown") (/ 1.0 (+ (/ (Utilities|Struct|BreakST_UnitStats _output_get) 100) (Variables|Default|GetAttacksPerSecond))))
      (Variables|/Script/Engine.CharacterMovementComponent|SetMaxWalkSpeed (Variables|Character|GetCharacterMovement) (* (+ (/ (Utilities|Struct|BreakST_UnitStats (Variables|Default|GetStats)) 100) 1.0) (Variables|Default|GetDefaultMovementSpeed))))))

(fn ConstructionScript)

(fn IsAnEnemy
  (params (ActorToCheck :type Actor%20Object%20Reference))
  (bind _array_element (Utilities|Array|ForEachLoopwithBreak (Variables|Default|GetEnemyTags) :!label _label)
    (:LoopBody
      (if (Utilities|Array|ContainsItem (Variables|/Script/Engine.Actor|GetTags ActorToCheck) _array_element)
        (LocalVariables|SetIsEnemy (Utilities|Array|ContainsItem (Variables|/Script/Engine.Actor|GetTags ActorToCheck) _array_element))
        (goto _label Break)))
    (:Completed
      (return (LocalVariables|GetIsEnemy)))))

(fn FindClosestEnemy
  (LocalVariables|SetClosestEnemy -1)
  (LocalVariables|SetClosestDistance 1e+05)
  (bind (_keypin _valuepin) (Utilities|Map|ForEachLoop(Map) (Variables|Default|GetSurroundingEnemies))
    (:then
      (if (< (Transformation|GetDistanceTo _valuepin self) (LocalVariables|GetClosestDistance))
        (LocalVariables|SetClosestEnemy _keypin)
        (LocalVariables|SetClosestDistance (Transformation|GetDistanceTo _valuepin self))))
    (:CompletedPin
      (return (LocalVariables|GetClosestEnemy) (.Value (Utilities|Map|Find (Variables|Default|GetSurroundingEnemies) (LocalVariables|GetClosestEnemy)))))))