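; Wave minion that auto-attacks nearby enemies, with spawn and death particle effects.
; An EnemyPerception overlap tracks tag-matched enemies and maintains the blackboard's AutoAttackTarget, falling back to the closest on exit.
; Attack damages BI_Attackable targets and holds IsAttacking through the cooldown; stat updates rescale walk speed and blackboard cooldown.
; Lethal damage only fires OnMinionDeath; a separate Kill event destroys the actor.
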(event OnComponentBeginOverlap(EnemyPerception)
  (params (OverlappedComponent :type Primitive%20Component%20Object%20Reference) (OtherActor :type Actor%20Object%20Reference) (OtherComp :type Primitive%20Component%20Object%20Reference) (OtherBodyIndex :type Integer) (bFromSweep :type Boolean) (SweepResult :type Hit%20Result%20Structure%20%28by%20ref%29))
  (bind _returnvalue (Utilities|Name|MakeLiteralName "AutoAttackTarget"))
  (bind _returnvalue_2 (AI|GetBlackboard 0))
  (if (CallFunction|IsAnEnemy OtherActor)
    (Utilities|Array|Add (Variables|Default|GetSurroundingEnemies) OtherActor)
    (Utilities|IsValid _returnvalue_2
      (:Is%20Valid
        (Utilities|IsValid (AI|Components|Blackboard|GetValueasObject _returnvalue_2 _returnvalue)
          (:Is%20Not%20Valid
            (AI|Components|Blackboard|SetValueasObject _returnvalue_2 _returnvalue OtherActor)))))))

(event OnComponentEndOverlap(EnemyPerception)
  (params (OverlappedComponent :type Primitive%20Component%20Object%20Reference) (OtherActor :type Actor%20Object%20Reference) (OtherComp :type Primitive%20Component%20Object%20Reference) (OtherBodyIndex :type Integer))
  (bind _returnvalue (Utilities|Name|MakeLiteralName "AutoAttackTarget"))
  (bind _returnvalue_2 (AI|GetBlackboard 0))
  (bind _returnvalue_3 (AI|Components|Blackboard|GetValueasObject _returnvalue_2 _returnvalue))
  (Utilities|Array|RemoveItem (Variables|Default|GetSurroundingEnemies) OtherActor)
  (Utilities|IsValid _returnvalue_2
    (:Is%20Valid
      (if (and (== OtherActor _returnvalue_3) (Utilities|IsValid _returnvalue_3))
        (if (Utilities|Array|IsNotEmpty (Variables|Default|GetSurroundingEnemies))
          (AI|Components|Blackboard|SetValueasObject _returnvalue_2 _returnvalue (CallFunction|FindClosestEnemy))
          (else
            (AI|Components|Blackboard|SetValueasObject _returnvalue_2 _returnvalue 0)))))))

(event EventAttack
  (params (Target :type Actor%20Object%20Reference))
  (bind _stats (Variables|Default|GetStats))
  (bind (_attackspeed _attackdamage) (Utilities|Struct|BreakST_UnitStats _stats))
  (bind _asbi_attackable (Utilities|Casting|CastToBI_Attackable Target))
  (Variables|Default|SetIsAttacking true)
  (Default|ReceiveDamage _asbi_attackable (* _attackdamage (Variables|Default|GetBaseAttackDamage)) self)
  (Utilities|FlowControl|Delay (/ 1.0 (+ (/ _attackspeed 100) (Variables|Default|GetAttacksPerSecond))))
  (Variables|Default|SetIsAttacking false))

(event EventInit
  (params (Stats :type ST%20Unit%20Stats%20Structure))
  (Variables|Default|SetStats Stats))

(event EventDamage
  (params (Damage :type Float%20%28double-precision%29) (DamageSource :type Actor%20Object%20Reference))
  (bind _output_get (Variables|Default|SetLife (- (Variables|Default|GetLife) Damage)))
  (if (<= _output_get 0.0)
    (Default|CallOnMinionDeath self DamageSource)))

(event EventKill
  (Effects|SpawnEmitteratLocation "/Game/FXVarietyPack/Particles/P_ky_hit2.P_ky_hit2" (Transformation|GetActorLocation))
  (Actor|DestroyActor))

(event EventBeginPlay
  (bind _returnvalue (Effects|SpawnEmitteratLocation "/Game/FXVarietyPack/Particles/P_ky_magicCircle1.P_ky_magicCircle1" (Transformation|GetActorLocation)))
  (Utilities|FlowControl|Delay 0.5)
  (Components|Activation|Deactivate _returnvalue))

(event EventUpdateStats
  (params (NewStats :type ST%20Unit%20Stats%20Structure))
  (bind _returnvalue (AI|GetBlackboard 0))
  (bind _output_get (Variables|Default|SetStats NewStats))
  (Utilities|IsValid _returnvalue
    (:Is%20Valid
      (AI|Components|Blackboard|SetValueasFloat _returnvalue (Utilities|Name|MakeLiteralName "AttackCooldown") (/ 1.0 (+ (/ (Utilities|Struct|BreakST_UnitStats _output_get) 100) (Variables|Default|GetAttacksPerSecond))))
      (Variables|/Script/Engine.CharacterMovementComponent|SetMaxWalkSpeed (Variables|Character|GetCharacterMovement) (* (+ (/ (Utilities|Struct|BreakST_UnitStats (Variables|Default|GetStats)) 100) 1.0) (Variables|Default|GetDefaultMovementSpeed))))))

(fn ConstructionScript)

(fn IsAnEnemy
  (params (ActorToCheck :type Actor%20Object%20Reference))
  (bind _array_element (Utilities|Array|ForEachLoopwithBreak (Variables|Default|GetEnemyTags) :!label _label)
    (:LoopBody
      (if (Utilities|Array|ContainsItem (Variables|/Script/Engine.Actor|GetTags ActorToCheck) _array_element)
        (LocalVariables|SetIsEnemy (Utilities|Array|ContainsItem (Variables|/Script/Engine.Actor|GetTags ActorToCheck) _array_element))
        (goto _label Break)))
    (:Completed
      (return (LocalVariables|GetIsEnemy)))))

(fn FindClosestEnemy
  (LocalVariables|SetClosestEnemy 0)
  (LocalVariables|SetClosestDistance 1e+05)
  (for _array_element (Variables|Default|GetSurroundingEnemies)
    (if (< (Transformation|GetDistanceTo _array_element self) (LocalVariables|GetClosestDistance))
      (LocalVariables|SetClosestEnemy _array_element)
      (LocalVariables|SetClosestDistance (Transformation|GetDistanceTo _array_element self))))
  (return (LocalVariables|GetClosestEnemy)))