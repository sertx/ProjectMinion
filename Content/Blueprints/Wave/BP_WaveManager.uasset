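; BP_WaveManager manages the player's wave of minions, spawning the starting group at random reachable points near the player character.
; It tracks each minion, shares unit stats with it and removes it through its death event.
; Passive items feed stat updates to all minions and fire change dispatchers.
; Movement orders and the auto-attack toggle are written to a Blackboard alongside the player reference, while SetAttackTarget is an empty stub.
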(event EventPostInit
  (params (PlayerCharacter :type BP%20Player%20Character%20Object%20Reference) (WaveManager :type BP%20Wave%20Manager%20Object%20Reference) (EnemyMinionsManager :type BP%20Enemy%20Minions%20Manager%20Object%20Reference) (ChampsManager :type Object%20Object%20Reference))
  (Variables|References|SetPlayer%20Char PlayerCharacter)
  (Variables|References|SetEnemyMinionsManager EnemyMinionsManager)
  (Init|SetupWave)
  (Init|SetupBlackboard))

(event EventInit
  (params (GameMode :type BP%20Swarm%20Gamemode%20Object%20Reference))
  (Variables|References|SetGame%20Mode GameMode))

(fn ConstructionScript)

(fn ClearWave
  (for _array_element (Variables|Default|GetMinions)
    (Actor|DestroyActor _array_element)))

(fn SetupWave
  (Init|ClearWave)
  (for _index (range 0 (Variables|Default|GetStartingWaveSize))
    (CallFunction|AddMinion)))

(fn SetAttackTarget)

(fn AddMinion
  (bind _returnvalue (Game|SpawnActorfromClass (Variables|Default|GetPlayerMinionClass) (Math|Transform|MakeTransform (.RandomLocation (AI|Navigation|GetRandomReachablePointinRadius (Transformation|GetActorLocation (Variables|References|GetPlayer%20Char)) 2e+02 0 0)) "0, 0, 0" "1.000000,1.000000,1.000000") "AdjustIfPossibleButAlwaysSpawn" "MultiplyWithRoot" 0 0))
  (bind _asbp_wave_minion (Utilities|Casting|CastToBP_WaveMinion _returnvalue))
  (Utilities|Array|Add (Variables|Default|GetMinions) _asbp_wave_minion)
  (Default|Init _asbp_wave_minion (Variables|Default|GetMinionStats))
  (EventDispatchers|BindEventtoOnUnitDeath _asbp_wave_minion (EventDispatchers|CreateEvent :!event OnUnitDeath)))

(fn RemoveMinion
  (params (Minion :type BP%20Unit%20Object%20Reference))
  (Utilities|Array|RemoveItem (Variables|Default|GetMinions) Minion)
  (Default|Kill Minion))

(fn SetupBlackboard
  (AI|Components|Blackboard|SetValueasObject (Variables|Default|GetBlackboard) (Utilities|Name|MakeLiteralName "PlayerCharacter") (Variables|References|GetPlayer%20Char)))

(fn UpdateStats
  (params (MinionStats :type ST%20Unit%20Stats%20Structure))
  (bind (_movementspeed _attackspeed _attackdamage) (Utilities|Struct|BreakST_UnitStats MinionStats))
  (bind _output_get (Variables|Default|SetMinionStats (Utilities|Struct|MakeST_UnitStats (+ _movementspeed (.MovementSpeed (Utilities|Struct|BreakST_UnitStats (Variables|Default|GetMinionStats)))) (+ _attackspeed (.AttackSpeed (Utilities|Struct|BreakST_UnitStats (Variables|Default|GetMinionStats)))) (+ _attackdamage (.AttackDamage (Utilities|Struct|BreakST_UnitStats (Variables|Default|GetMinionStats)))))))
  (for _array_element (Variables|Default|GetMinions)
    (Default|UpdateStats _array_element _output_get))
  (Default|CallStatsUpdated (Variables|Default|GetMinionStats)))

(fn SetMovementTarget
  (params (VectorValue :type Vector))
  (AI|Components|Blackboard|SetValueasVector (Variables|Default|GetBlackboard) (Utilities|Name|MakeLiteralName "MovementTarget") VectorValue)
  (AI|Components|Blackboard|SetValueasBool (Variables|Default|GetBlackboard) (Utilities|Name|MakeLiteralName "HasMovementOrder") true))

(fn ToggleAutoAttack
  (params (AutoAttack :type Boolean))
  (Variables|Default|SetAutoAttack AutoAttack)
  (AI|Components|Blackboard|SetValueasBool (Variables|Default|GetBlackboard) (Utilities|Name|MakeLiteralName "AutoAttack") AutoAttack))

(fn AddPassiveItem
  (params (NewItem :type ST%20Passive%20Item%20Structure))
  (Utilities|Array|Add (Variables|Default|GetPassiveItems) NewItem)
  (Updates|UpdateStats (Utilities|Struct|BreakST_PassiveItem NewItem))
  (Default|CallPassiveItemsChanged (Variables|Default|GetPassiveItems)))

(fn OnUnitDeath
  (params (DyingUnit :type BP%20Unit%20Object%20Reference) (DamagingUnit :type BP%20Unit%20Object%20Reference))
  (CallFunction|RemoveMinion DyingUnit))