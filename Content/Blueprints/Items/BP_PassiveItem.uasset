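; BP_PassiveItem is a world pickup actor that stores the passive item passed to it through Init.
; On spawn, a radial impulse from just below pops its Sphere upward, while Tick spins the Cube with small randomized rotations.
; PickUp fires a much stronger impulse to launch it, then destroys the actor after a short delay.
; Highlight is an empty event, and PickUp does not itself grant the item.
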(event Custom|Init
  (params (PassiveItem :type ST%20Passive%20Item%20Structure))
  (Variables|Default|SetPassiveItem PassiveItem))

(event Custom|Highlight)

(event Custom|PickUp
  (Class|PhysicsObjectBlueprintLibrary|ApplyRadialImpulse (Variables|Default|GetSphere) (- (Transformation|GetActorLocation) "0.000000,0.000000,30.000000") 2e+02 3.5e+03 "RIF_Constant" false 0.0 true 0.0 1.0)
  (Utilities|FlowControl|Delay 2.0)
  (Actor|DestroyActor))

(event EventTick
  (params (DeltaSeconds :type Float%20%28single-precision%29))
  (Transformation|AddWorldRotation (Variables|Default|GetCube) (* (Math|Conversions|RotationFromXVector (Math|Vector|VectorGetAbs (Math|Random|RandomUnitVector))) DeltaSeconds) false false))

(event EventBeginPlay
  (Class|PhysicsObjectBlueprintLibrary|ApplyRadialImpulse (Variables|Default|GetSphere) (- (Transformation|GetActorLocation) "0.000000,0.000000,30.000000") 2e+02 7.5e+02 "RIF_Constant" false 0.0 true 0.0 1.0))

(fn ConstructionScript)